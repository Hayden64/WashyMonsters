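; BP_WashingMachine is an interactable washer that turns the player's held dirty laundry into wet laundry through a chain of minigames.
; Interact opens the washing minigame, and callback events swap in fill-bar and temp widgets, each referencing the machine.
; StartWashing takes the load and runs a timer, which Tick feeds to a timer bar widget.
; Items are colon-delimited strings; finishing appends Temperature, and Interact handles pickup.
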(event `/Game/Blueprints/I_Interact.Interact`
  (bind _returnvalue (`GameplayStatics.GetPlayerController` 0))
  (bind _contents (`self.Contents`))
  (bind _returnvalue_2 (`KismetStringLibrary.ParseIntoArray` _contents ":"))
  (bind _asbp_player (cast `/Game/Blueprints/BP_Player` (`GameplayStatics.GetPlayerCharacter` 0)))
  (bind _holding (`/Game/Blueprints/BP_Player.Holding` _asbp_player))
  (bind _returnvalue_3 (`KismetStringLibrary.ParseIntoArray` _holding ":"))
  (if (or (not (== (`KismetArrayLibrary.Array_Length` _returnvalue_3) 2)) (not (`KismetStringLibrary.EqualEqual_StrStr` (`self.Contents`))))
    (if (and (== (`KismetArrayLibrary.Array_Length` _returnvalue_2) 3) (`KismetStringLibrary.EqualEqual_StrStr` _holding))
      (switch `string` (`|GetArrayItem` _returnvalue_2)
        (:`WetLaundry`
          (bind _output_get (set `/Game/Blueprints/BP_Player.Holding` _contents _asbp_player))
          (`KismetSystemLibrary.PrintString` _output_get)
          (set `self.Contents` ""))))
    (else
      (switch `string` (`|GetArrayItem` _returnvalue_3)
        (:`DirtyLaundry`
          (bind _returnvalue_4 (`|CreateWidget` "/Game/WashingMachineMinigame/DragableWidgets/WB_WashingMinigame.WB_WashingMinigame_C"))
          (set `/Game/WashingMachineMinigame/DragableWidgets/WB_WashingMinigame.WashingMachineRef` self _returnvalue_4)
          (`UserWidget.AddToViewport` _returnvalue_4 0)
          (set `PlayerController.bShowMouseCursor` true _returnvalue)
          (`WidgetBlueprintLibrary.SetInputMode_UIOnlyEx` _returnvalue null))))))

(event `StartDialGame`
  (`AudioComponent.Play` (`self.Audio`) 0.0)
  (`Widget.RemoveFromParent` (stale `/Game/Blueprints/I_Interact.Interact` _returnvalue_4))
  (`KismetSystemLibrary.PrintString` "AddWidget")
  (bind _returnvalue (`|CreateWidget` "/Game/WashingMachineMinigame/WG_FillBar.WG_FillBar_C"))
  (set `/Game/WashingMachineMinigame/WG_FillBar.WashingMachineRef` self _returnvalue)
  (`UserWidget.AddToViewport` _returnvalue 0))

(event `StartDetergentGame`
  (`Widget.RemoveFromParent` (stale `StartDialGame` _returnvalue))
  (`KismetSystemLibrary.PrintString` "AddWidget")
  (bind _returnvalue (`|CreateWidget` "/Game/WashingMachineMinigame/ChangeTemp/BP_TempMiniGame.BP_TempMiniGame_C"))
  (set `/Game/WashingMachineMinigame/ChangeTemp/BP_TempMiniGame.WashingMachineRef` self _returnvalue)
  (`UserWidget.AddToViewport` _returnvalue 0))

(event `StartWashing`
  (`Widget.RemoveFromParent` (stale `StartDetergentGame` _returnvalue))
  (set `PlayerController.bShowMouseCursor` false (`GameplayStatics.GetPlayerController` 0))
  (bind _asbp_player (cast `/Game/Blueprints/BP_Player` (`GameplayStatics.GetPlayerCharacter` 0)))
  (set `/Game/Blueprints/BP_Player.CanMove` true _asbp_player)
  (bind _output_get (set `self.Contents` (`/Game/Blueprints/BP_Player.Holding` (stale `/Game/Blueprints/I_Interact.Interact` _asbp_player))))
  (`KismetSystemLibrary.PrintString` "Washing")
  (set `/Game/Blueprints/BP_Player.Holding` "" (stale `/Game/Blueprints/I_Interact.Interact` _asbp_player))
  (bind _returnvalue (`KismetSystemLibrary.K2_SetTimerDelegate` (delegate `FinishedWashing`) (`self.TimeToWash`)))
  (set `self.WashingTimer` _returnvalue)
  (bind _returnvalue_2 (`|GenericCreateObject` "/Game/Monsters/WB_TimerBar.WB_TimerBar_C"))
  (bind _output_get_2 (set `self.WashTimerWidgetRef` _returnvalue_2))
  (`WidgetComponent.SetWidget` (`self.TimerWidget`) _output_get_2))

(event `self.ReceiveTick`
  (params (DeltaSeconds :type "Float (single-precision)"))
  (bind _washingtimer (`self.WashingTimer`))
  (if (`KismetSystemLibrary.K2_IsTimerActiveHandle` _washingtimer)
    (set `/Game/Monsters/WB_TimerBar.Timer Value` (/ (* (`KismetSystemLibrary.K2_GetTimerRemainingTimeHandle` _washingtimer) 10.0) 100.0) (`self.WashTimerWidgetRef`))))

(event `FinishedWashing`
  (set `self.Contents` (`KismetStringLibrary.Concat_StrStr` "WetLaundry:" (`|GetArrayItem` (`KismetStringLibrary.ParseIntoArray` (stale `StartWashing` _output_get) ":") 1) ":" (`self.Temperature`)))
  (set `self.Temperature` "")
  (`KismetSystemLibrary.PrintString` "FinishedWashing")
  (`GameplayStatics.PlaySound2D` "/Game/Felix/SFX_WasherComplete.SFX_WasherComplete" 1.0 1.0 0.0 null null))

(fn `UserConstructionScript`)