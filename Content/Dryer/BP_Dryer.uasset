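; Dryer actor that takes wet laundry from the player, dries it on a short timer and hands back clean laundry.
; Interact swaps colon-delimited item strings between the character's Holding and the dryer's Contents, branching on the type prefix.
; When the timer ends, FinishedDrying rewrites the prefix, keeping the second field.
; Tick feeds remaining time to a WB_MonsterTimer widget shown on the Timer component.
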(event `/Game/ThirdPerson/Blueprints/I_Interact.Interact`
  (bind _contents (`self.Contents`))
  (bind _returnvalue (`KismetStringLibrary.ParseIntoArray` _contents ":"))
  (bind _asbp_third_person_character (cast `/Game/ThirdPerson/Blueprints/BP_ThirdPersonCharacter` (`GameplayStatics.GetPlayerCharacter` 0)))
  (bind _holding (`/Game/ThirdPerson/Blueprints/BP_ThirdPersonCharacter.Holding` _asbp_third_person_character))
  (bind _returnvalue_2 (`KismetStringLibrary.ParseIntoArray` _holding ":"))
  (if (or (not (== (`KismetArrayLibrary.Array_Length` _returnvalue_2) 2)) (not (`KismetStringLibrary.EqualEqual_StrStr` (`self.Contents`))))
    (if (and (== (`KismetArrayLibrary.Array_Length` _returnvalue) 2) (`KismetStringLibrary.EqualEqual_StrStr` _holding))
      (switch `string` (`|GetArrayItem` _returnvalue)
        (:`CleanLaundry`
          (bind _output_get (set `/Game/ThirdPerson/Blueprints/BP_ThirdPersonCharacter.Holding` _contents _asbp_third_person_character))
          (`KismetSystemLibrary.PrintString` _output_get)
          (set `self.Contents` ""))))
    (else
      (switch `string` (`|GetArrayItem` _returnvalue_2)
        (:`WetLaundry`
          (bind _output_get_2 (set `self.Contents` _holding))
          (`KismetSystemLibrary.PrintString` "Drying")
          (set `/Game/ThirdPerson/Blueprints/BP_ThirdPersonCharacter.Holding` "" _asbp_third_person_character)
          (bind _returnvalue_3 (`KismetSystemLibrary.K2_SetTimerDelegate` (delegate `FinishedDrying`) 5.0))
          (set `self.dyertimer` _returnvalue_3)
          (bind _returnvalue_4 (`|GenericCreateObject` "/Game/Monsters/WB_MonsterTimer.WB_MonsterTimer_C"))
          (bind _output_get_3 (set `self.dryerwidgetref` _returnvalue_4))
          (`WidgetComponent.SetWidget` (`self.Timer`) _output_get_3))))))

(event `FinishedDrying`
  (set `self.Contents` (`KismetStringLibrary.Concat_StrStr` "CleanLaundry:" (`|GetArrayItem` (`KismetStringLibrary.ParseIntoArray` (stale `/Game/ThirdPerson/Blueprints/I_Interact.Interact` _output_get_2) ":") 1)))
  (`KismetSystemLibrary.PrintString` "Finished drying"))

(event `self.ReceiveTick`
  (params (DeltaSeconds :type "Float (single-precision)"))
  (bind _dyertimer (`self.dyertimer`))
  (if (`KismetSystemLibrary.K2_IsTimerActiveHandle` _dyertimer)
    (set `/Game/Monsters/WB_MonsterTimer.Timer Value` (/ (* (`KismetSystemLibrary.K2_GetTimerRemainingTimeHandle` _dyertimer) 20.0) 100.0) (`self.dryerwidgetref`))))

(fn `UserConstructionScript`)