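; Vending machine actor that randomly breaks down during work shifts, giving the player a timed minigame to fix it.
; BP_ServiceBell shift events start and stop the random breakdown timer; a breakdown starts a countdown shown on a timer bar widget.
; Interacting during a breakdown disables player input and opens WG_VendingMachine, with events here to clear the countdown and restore control.
; Running out of time damages the player and schedules another breakdown.
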(event `self.ReceiveBeginPlay`
  ;[1 1 1] Initialise
  (bind _asbp_player (cast `/Game/Blueprints/BP_Player` (`GameplayStatics.GetPlayerPawn` 0)))
  (set `self.AsPlayer` _asbp_player)
  (bind _returnvalue (`GameplayStatics.GetActorOfClass` "/Game/Blueprints/BP_ServiceBell.BP_ServiceBell_C"))
  (bind _output_get (set `self.AsServiceBell` _returnvalue))
  (add `/Game/Blueprints/BP_ServiceBell.OnShiftStarted` _output_get (`|CreateDelegate` :!event `ShiftStarted`))
  (add `/Game/Blueprints/BP_ServiceBell.OnShiftEnded` _output_get (`|CreateDelegate` :!event `ShiftEnded`)))

(event `/Game/Blueprints/I_Interact.Interact`
  (bind _returnvalue (`GameplayStatics.GetPlayerController` 0))
  ;[1 1 1] Interact
  (if (`self.Minigame`)
    (`self.DisableInput` (`self.AsPlayer`) _returnvalue)
    (bind _returnvalue_2 (`|CreateWidget` "/Game/Widgets/WG_VendingMachine.WG_VendingMachine_C" _returnvalue))
    (bind _output_get (set `self.AsVendingWidget` _returnvalue_2))
    (`UserWidget.AddToViewport` _output_get 0)
    (set `/Game/Widgets/WG_VendingMachine.AsVendingMachine` self _output_get)))

(event `CreateBreakdownTimer`
  ;[1 1 1] Create breakdown timer
  (bind _returnvalue (`KismetSystemLibrary.K2_SetTimerDelegate` (`|CreateDelegate` :!event `CreateMinigameTimer`) (`KismetMathLibrary.RandomFloatInRange` (`self.BreakdownMinimum`) (`self.BreakdownMaximum`)))) ; Vending machine breakdown timer
  (set `self.BreakdownTimer` _returnvalue))

(event `CreateMinigameTimer`
  (bind _timerwidget (`self.TimerWidget`))
  ;[1 1 1] Set minigame timer
  (set `self.Minigame` true)
  (bind _returnvalue (`KismetSystemLibrary.K2_SetTimerDelegate` (`|CreateDelegate` :!event `DamagePlayer`) (`self.MinigameTime`))) ; Time to complete minigame before angry
  (set `self.MinigameTimer` _returnvalue)
  (bind _returnvalue_2 (`|GenericCreateObject` "/Game/Widgets/WB_TimerBarBlue.WB_TimerBarBlue_C"))
  (bind _output_get (set `self.AsTimerBar` _returnvalue_2))
  (`WidgetComponent.SetWidget` _timerwidget _output_get)
  (`SceneComponent.SetVisibility` _timerwidget true false)
  (bind _returnvalue_3 (`KismetSystemLibrary.K2_SetTimerDelegate` (`|CreateDelegate` :!event `UpdateTimerWidget`) 0.05 true))
  (set `self.UpdateTimerWidgetTimer` _returnvalue_3))

(event `ResetViewport`
  ;[1 1 1] Reset hud once minigame is completed
  (`Widget.RemoveFromParent` (`self.AsVendingWidget`))
  (set `self.Minigame` false)
  (`self.EnableInput` (`self.AsPlayer`) (`GameplayStatics.GetPlayerController` 0))
  (if (`/Game/Blueprints/BP_ServiceBell.ShiftStarted` (`self.AsServiceBell`))
    (`self.CreateBreakdownTimer`)))

(event `ClearMinigameTimer`
  ;[1 1 1] Clear minigame timer
  (`KismetSystemLibrary.K2_ClearAndInvalidateTimerHandle` (`self.MinigameTimer`))
  (`KismetSystemLibrary.K2_ClearAndInvalidateTimerHandle` (`self.UpdateTimerWidgetTimer`))
  (`SceneComponent.SetVisibility` (`self.TimerWidget`) false false)
  (`GameplayStatics.PlaySound2D` "/Game/Sounds/SFX/SFX_CandyFalling.SFX_CandyFalling" 1.0 1.0 0.0 null null))

(event `UpdateTimerWidget`
  ;[1 1 1] Update timer with minigame time left as percentage
  (`ProgressBar.SetPercent` (`/Game/Widgets/WB_TimerBarBlue.ProgressBar` (`self.AsTimerBar`)) (/ (`KismetSystemLibrary.K2_GetTimerRemainingTimeHandle` (`self.MinigameTimer`)) (`self.MinigameTime`))))

(event `DamagePlayer`
  ;[1 1 1] Damage player
  (`GameplayStatics.ApplyDamage` (`self.AsPlayer`) 25.0)
  (`GameplayStatics.PlaySound2D` "/Game/Sounds/SFX/SFX_MonsterSad.SFX_MonsterSad" 1.0 1.0 0.0 null null)
  (`self.CreateBreakdownTimer`))

(event `ShiftStarted`
  ;[1 1 1] Shift started
  (`self.CreateBreakdownTimer`))

(event `ShiftEnded`
  ;[1 1 1] Shift ended
  (`KismetSystemLibrary.K2_ClearAndInvalidateTimerHandle` (`self.BreakdownTimer`)))

(fn `UserConstructionScript`)