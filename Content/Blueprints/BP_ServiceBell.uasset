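; BP_ServiceBell is an interactable bell that starts a timed shift and tracks the level number.
; Interacting while no shift runs spawns BP_MonsterSpawner, swaps the cone for a W_LevelTimer countdown display, starts one-minute shift and per-second timers, and broadcasts the start.
; EndShift stops spawning, restores the cone, clears both timers, increments the level and broadcasts the end.
; UpdateTimerWidget shows the rounded remaining shift time.
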(event `/Game/Blueprints/I_Interact.Interact`
  ;[1 1 1] Spawn monster spawner and start level timer if level is not already started
  (if (not (`self.ShiftStarted`))
    (`SceneComponent.SetVisibility` (`self.Cone`) false false)
    (`SceneComponent.SetVisibility` (`self.TimerDisplay`) true false)
    (bind _returnvalue (`|SpawnActorFromClass` "/Game/Blueprints/BP_MonsterSpawner.BP_MonsterSpawner_C" (`KismetMathLibrary.MakeTransform` (-1542.0 923.0 0.0)) "Undefined" "MultiplyWithRoot" self null))
    (set `self.MonsterSpawnerRef` _returnvalue)
    (bind _returnvalue_2 (`KismetSystemLibrary.K2_SetTimerDelegate` (`|CreateDelegate` :!event `EndShift`) 60.0))
    (set `self.ShiftTimer` _returnvalue_2)
    (bind _returnvalue_3 (`|GenericCreateObject` "/Game/Widgets/W_LevelTimer.W_LevelTimer_C"))
    (bind _output_get (set `self.TimerWidget` _returnvalue_3))
    (`WidgetComponent.SetWidget` (`self.TimerDisplay`) _output_get)
    (bind _returnvalue_4 (`KismetSystemLibrary.K2_SetTimerDelegate` (`|CreateDelegate` :!event `UpdateTimerWidget`) 1.0 true))
    (set `self.UpdateWidgetTimer` _returnvalue_4)
    (set `self.ShiftStarted` true)
    (`self.UpdateTimerWidget`)
    (`self.OnShiftStarted`)))

(event `EndShift`
  ;[1 1 1] End shift, increment level
  (`/Game/Blueprints/BP_MonsterSpawner.EndSpawning` (`self.MonsterSpawnerRef`))
  (`SceneComponent.SetVisibility` (`self.Cone`) true false)
  (`SceneComponent.SetVisibility` (`self.TimerDisplay`) false false)
  (set `self.ShiftStarted` false)
  (set `self.Level` (+ (`self.Level`) 1.0))
  (`KismetSystemLibrary.K2_ClearAndInvalidateTimerHandle` (`self.ShiftTimer`))
  (`KismetSystemLibrary.K2_ClearAndInvalidateTimerHandle` (`self.UpdateWidgetTimer`))
  (`self.OnShiftEnded`))

(event `UpdateTimerWidget`
  ;[1 1 1] Update timer display
  (`TextBlock.SetText` (`/Game/Widgets/W_LevelTimer.TextBlock_Time` (`self.TimerWidget`)) (`KismetTextLibrary.Conv_IntToText` (`KismetMathLibrary.Round` (`KismetSystemLibrary.K2_GetTimerRemainingTimeHandle` (`self.ShiftTimer`))))))

(fn `UserConstructionScript`)