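; BP_BrokenMachine is an interactable machine that opens the cleaning minigame.
; Interact creates a W_CleaningGame widget, stores it, adds it to the viewport, then shows the cursor and switches to UI-only input to stop player movement.
; RemoveWidget removes the stored widget, hides the cursor and restores game-only input so the player can move again.
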(event `/Game/ThirdPerson/Blueprints/I_Interact.Interact`
  (bind _returnvalue (`GameplayStatics.GetPlayerController` 0))
  ;[0.5819 1 0.5801] Adds widget to viewport and stops player from moving - Hayden
  (bind _returnvalue_2 (`|CreateWidget` "/Game/Hayden/CleaningMiniGame/W_CleaningGame.W_CleaningGame_C"))
  (bind _output_get (set `self.CleaningMinigame` _returnvalue_2))
  (`UserWidget.AddToViewport` _output_get 0)
  (set `PlayerController.bShowMouseCursor` true _returnvalue)
  (`WidgetBlueprintLibrary.SetInputMode_UIOnlyEx` _returnvalue null))

(event `Remove Widget`
  (bind _returnvalue (`GameplayStatics.GetPlayerController` 0))
  ;[0.5318 1 0.5496] Removes the widget from the screen and allows the player to move - Hayden
  (`Widget.RemoveFromParent` (`self.CleaningMinigame`))
  (set `PlayerController.bShowMouseCursor` false _returnvalue)
  (`WidgetBlueprintLibrary.SetInputMode_GameOnly` _returnvalue))

(fn `UserConstructionScript`)