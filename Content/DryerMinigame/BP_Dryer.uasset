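; BP_Dryer is an interactable dryer in a laundry game that turns the player's wet laundry clean and hands it back to an empty-handed player.
; Drying runs on a timer, with a looping timer updating a progress bar widget and a sound on completion.
; A randomly timed breakdown shows an alert and redirects interaction to a UI-only cleaning minigame, whose removal restores player control and reschedules the next breakdown.
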(event `self.ReceiveBeginPlay`
  ;[1 1 1] Initialise
  (bind _asbp_player (cast `/Game/Blueprints/BP_Player` (`GameplayStatics.GetPlayerCharacter` 0)))
  (set `self.AsPlayer` _asbp_player)
  (set `self.AsPlayerController` (`GameplayStatics.GetPlayerController` 0))
  (bind _returnvalue (`KismetSystemLibrary.K2_SetTimerDelegate` (`|CreateDelegate` :!event `TriggerBreakdown`) (`KismetMathLibrary.RandomFloatInRange` (`self.BreakdownMinimum`) (`self.BreakdownMaximum`))))
  (set `self.BreakdownTimer` _returnvalue)
  (bind _returnvalue_2 (`|GenericCreateObject` "/Game/Widgets/W_TimerBarBlue.W_TimerBarBlue_C"))
  (bind _output_get (set `self.AsDryTimerWidget` _returnvalue_2))
  (`WidgetComponent.SetWidget` (`self.DryTimerWidget`) _output_get)
  (`WidgetComponent.SetTintColorAndOpacity` (`self.DryTimerWidget`) (struct :`R` 0.004252 :`G` 1.0 :`A` 1.0)))

(event `/Game/Blueprints/I_Interact.Interact`
  ;[1 1 1] Interact and call either regular or breakdown event
  (if (not (`self.IsBreakdown`))
    (`self.BeginDrying`)
    (else
      (`self.Breakdown`))))

(event `TriggerBreakdown`
  ;[1 1 1] Trigger breakdown when timer expires
  (set `self.IsBreakdown` true)
  (`SceneComponent.SetVisibility` (`self.BreakdownAlert`) true false))

(event `Breakdown`
  (bind _asplayercontroller (`self.AsPlayerController`))
  ;[1 1 1] Start breakdown minigame
  (bind _returnvalue (`|CreateWidget` "/Game/DryerMinigame/W_CleaningGame.W_CleaningGame_C"))
  (bind _output_get (set `self.AsCleaningWidget` _returnvalue))
  (set `/Game/DryerMinigame/W_CleaningGame.AsDryer` self _output_get)
  (`UserWidget.AddToViewport` _output_get 0)
  (`Controller.SetIgnoreMoveInput` _asplayercontroller true)
  (set `PlayerController.bShowMouseCursor` true _asplayercontroller)
  (`WidgetBlueprintLibrary.SetInputMode_UIOnlyEx` _asplayercontroller null))

(event `Remove Widget`
  (bind _asplayercontroller (`self.AsPlayerController`))
  ;[1 1 1] End breakdown minigame
  (`Widget.RemoveFromParent` (`self.AsCleaningWidget`))
  (`Controller.SetIgnoreMoveInput` _asplayercontroller false)
  (set `PlayerController.bShowMouseCursor` false _asplayercontroller)
  (`WidgetBlueprintLibrary.SetInputMode_GameOnly` _asplayercontroller)
  (set `self.IsBreakdown` false)
  (bind _returnvalue (`KismetSystemLibrary.K2_SetTimerDelegate` (`|CreateDelegate` :!event `TriggerBreakdown`) (`KismetMathLibrary.RandomFloatInRange` (`self.BreakdownMinimum`) (`self.BreakdownMaximum`))))
  (set `self.BreakdownTimer` _returnvalue)
  (`SceneComponent.SetVisibility` (`self.BreakdownAlert`) false false))

(event `BeginDrying`
  (bind (_currentlaundry_owner _currentlaundry_laundrystate) (break `/Game/Blueprints/S_Laundry` (`self.CurrentLaundry`)))
  (bind (_currentlaundry_owner_2 _currentlaundry_laundrystate_2) (break `/Game/Blueprints/S_Laundry` (`/Game/Blueprints/BP_Player.CurrentLaundry` (`self.AsPlayer`))))
  ;[1 1 1] Interact when not breakdown
  (switch `/Game/Blueprints/E_LaundryState` _currentlaundry_laundrystate_2 ; Player laundry
    (:`NewEnumerator0`
      (switch `/Game/Blueprints/E_LaundryState` _currentlaundry_laundrystate ; Dryer laundry
        (:`NewEnumerator3`
          (set `/Game/Blueprints/BP_Player.CurrentLaundry` (`self.CurrentLaundry`) (`self.AsPlayer`))
          (`SceneComponent.SetVisibility` (`self.DryTimerWidget`) false false))))
    (:`NewEnumerator2`
      (set `self.CurrentLaundry` (`/Game/Blueprints/BP_Player.CurrentLaundry` (`self.AsPlayer`)))
      (set `/Game/Blueprints/BP_Player.CurrentLaundry` (struct) (`self.AsPlayer`)) ; Empty player laundry
      (bind _returnvalue (`KismetSystemLibrary.K2_SetTimerDelegate` (`|CreateDelegate` :!event `FinishedDrying`) (`self.DryTimerLength`)))
      (set `self.DryTimer` _returnvalue)
      (`SceneComponent.SetVisibility` (`self.DryTimerWidget`) true false)
      (bind _returnvalue_2 (`KismetSystemLibrary.K2_SetTimerDelegate` (`|CreateDelegate` :!event `UpdateDryTimer`) 0.05 true))
      (set `self.UpdateDryWidgetTimer` _returnvalue_2))))

(event `FinishedDrying`
  (bind (_currentlaundry_owner _currentlaundry_laundrystate _currentlaundry_temperature) (break `/Game/Blueprints/S_Laundry` (`self.CurrentLaundry`)))
  ;[1 1 1] Finished drying
  (`KismetSystemLibrary.K2_ClearAndInvalidateTimerHandle` (`self.DryTimer`))
  (`KismetSystemLibrary.K2_ClearAndInvalidateTimerHandle` (`self.UpdateDryWidgetTimer`))
  (set `self.CurrentLaundry` (make `/Game/Blueprints/S_Laundry` _currentlaundry_owner "NewEnumerator3" _currentlaundry_temperature))
  (`GameplayStatics.PlaySound2D` "/Game/Sounds/SFX/SFX_DryerComplete.SFX_DryerComplete" 1.0 1.0 0.0 null null))

(event `UpdateDryTimer`
  ;[1 1 1] Update dry timer
  (`ProgressBar.SetPercent` (`/Game/Widgets/W_TimerBarBlue.ProgressBar` (`self.AsDryTimerWidget`)) (/ (`KismetSystemLibrary.K2_GetTimerRemainingTimeHandle` (`self.DryTimer`)) (`self.DryTimerLength`))))

(fn `UserConstructionScript`)