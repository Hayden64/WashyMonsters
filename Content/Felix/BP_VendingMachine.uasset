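; BP_VendingMachine is an interactable vending machine that opens its own menu for the player.
; Interact disables the third-person character's movement, shows WG_VendingMachine with a reference back to the machine, and plays MSC_Goblin on the Goblin audio component.
; ResetViewport undoes this by restoring movement, removing the widget and stopping the sound.
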(event `/Game/ThirdPerson/Blueprints/I_Interact.Interact`
  (bind _goblin (`self.Goblin`))
  (bind _asbp_third_person_character (cast `/Game/ThirdPerson/Blueprints/BP_ThirdPersonCharacter` (`GameplayStatics.GetPlayerCharacter` 0)))
  (set `/Game/ThirdPerson/Blueprints/BP_ThirdPersonCharacter.CanMove` false _asbp_third_person_character)
  (bind _returnvalue (`|CreateWidget` "/Game/Felix/WG_VendingMachine.WG_VendingMachine_C" (`GameplayStatics.GetPlayerController` 0)))
  (`UserWidget.AddToViewport` _returnvalue 0)
  (set `/Game/Felix/WG_VendingMachine.VendingMachineRef` self _returnvalue)
  (`AudioComponent.SetSound` _goblin "/Game/Felix/MSC_Goblin.MSC_Goblin")
  (`AudioComponent.Play` _goblin 0.0))

(event `ResetViewport`
  (set `/Game/ThirdPerson/Blueprints/BP_ThirdPersonCharacter.CanMove` true (stale `/Game/ThirdPerson/Blueprints/I_Interact.Interact` _asbp_third_person_character))
  (`Widget.RemoveFromParent` (stale `/Game/ThirdPerson/Blueprints/I_Interact.Interact` _returnvalue))
  (`AudioComponent.Stop` (`self.Goblin`)))

(fn `UserConstructionScript`)