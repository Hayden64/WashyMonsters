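; BP_Upgrade is an interactable actor that puts the player into a machine-placement mode.
; Interact switches the view to BP_CameraTest, stops character movement, shows W_PlaceMachine and the cursor, and enables input on the actor.
; Left click traces from the mouse with persistent debug drawing and spawns BP_BrokenMachine at the hit location, without checking for a hit.
; RemoveUI reverses the widget, cursor, movement, camera and input changes.
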(event `/Game/ThirdPerson/Blueprints/I_Interact.Interact`
  ;[1 1 1] Changes Camera (test whilst camera isnt fixed) - Hayden
  (bind _returnvalue (`GameplayStatics.GetActorOfClass` "/Game/Hayden/Upgrade/BP_CameraTest.BP_CameraTest_C"))
  (`PlayerController.SetViewTargetWithBlend` (`PlayerState.GetPlayerController` (`Pawn.PlayerState` (`GameplayStatics.GetPlayerCharacter` 0))) _returnvalue 0.0 "VTBlend_Linear" 0.0 false)
  (bind _returnvalue_2 (`GameplayStatics.GetActorOfClass` "/Game/ThirdPerson/Blueprints/BP_ThirdPersonCharacter.BP_ThirdPersonCharacter_C"))
  (set `/Game/ThirdPerson/Blueprints/BP_ThirdPersonCharacter.CanMove` false _returnvalue_2)
  (bind _returnvalue_3 (`|CreateWidget` "/Game/Hayden/Upgrade/W_PlaceMachine.W_PlaceMachine_C"))
  (`UserWidget.AddToViewport` _returnvalue_3 0)
  (set `PlayerController.bShowMouseCursor` true (`GameplayStatics.GetPlayerController` 0))
  (`self.EnableInput` (`GameplayStatics.GetPlayerController` 0)))

(event `RemoveUI`
  ;[1 1 1] Reverts everything back to normal - Hayden
  (`Widget.RemoveFromParent` (stale `/Game/ThirdPerson/Blueprints/I_Interact.Interact` _returnvalue_3))
  (set `PlayerController.bShowMouseCursor` false (`GameplayStatics.GetPlayerController` 0))
  (bind _returnvalue (`GameplayStatics.GetActorOfClass` "/Game/ThirdPerson/Blueprints/BP_ThirdPersonCharacter.BP_ThirdPersonCharacter_C"))
  (set `/Game/ThirdPerson/Blueprints/BP_ThirdPersonCharacter.CanMove` true _returnvalue)
  (bind _returnvalue_2 (`GameplayStatics.GetActorOfClass` "/Game/ThirdPerson/Blueprints/BP_ThirdPersonCharacter.BP_ThirdPersonCharacter_C"))
  (`PlayerController.SetViewTargetWithBlend` (`PlayerState.GetPlayerController` (`Pawn.PlayerState` (`GameplayStatics.GetPlayerCharacter` 0))) _returnvalue_2 0.0 "VTBlend_Linear" 0.0 false)
  (`self.DisableInput` (`GameplayStatics.GetPlayerController` 0)))

(event `Key|LeftMouseButton` :paused true
  (params (Key :type "Key Structure"))
  (bind (_worldlocation _worlddirection) (`PlayerController.DeprojectMousePositionToWorld` (`GameplayStatics.GetPlayerController` 0)))
  ;[1 1 1] creates linetrace from mouse location - Hayden
  (:`Pressed`
    (bind _outhit (`KismetSystemLibrary.LineTraceSingle` :`Start` _worldlocation :`End` (+ _worldlocation (* _worlddirection 5000000.0)) :`TraceChannel` "TraceTypeQuery1" :`DrawDebugType` "Persistent"))
    (`|SpawnActorFromClass` "/Game/Hayden/CleaningMiniGame/BP_BrokenMachine.BP_BrokenMachine_C" (`KismetMathLibrary.MakeTransform` (`.Location` (`GameplayStatics.BreakHitResult` _outhit))) "Undefined" "MultiplyWithRoot" null null)))

(fn `UserConstructionScript`)