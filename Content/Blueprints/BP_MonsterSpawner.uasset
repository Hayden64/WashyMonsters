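; Monster spawner owned by a BP_ServiceBell that spawns BP_Monster actors during the bell's shifts.
; Shift start spawns one immediately and starts a looping timer that quickens with bell level, while shift end clears it.
; The monster count is capped by level and a hard limit, and each spawn retries random picks for a counter slot and ID.
; A monster-left event lowers the count and frees its slot.
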(event `self.ReceiveBeginPlay`
  ;[1 1 1] Initialise
  (bind _asbp_service_bell (cast `/Game/Blueprints/BP_ServiceBell` (`self.GetOwner`)))
  (bind _output_get (set `self.AsBell` _asbp_service_bell))
  (add `/Game/Blueprints/BP_ServiceBell.OnShiftStarted` _output_get (`|CreateDelegate` :!event `BeginSpawning`))
  (add `/Game/Blueprints/BP_ServiceBell.OnShiftEnded` _output_get (`|CreateDelegate` :!event `EndSpawning`)))

(event `BeginSpawning`
  ;[1 1 1] Spawn monsters when shift starts
  (bind _returnvalue (`KismetSystemLibrary.K2_SetTimerDelegate` (`|CreateDelegate` :!event `SpawnMonster`) (/ 15.0 (`/Game/Blueprints/BP_ServiceBell.Level` (`self.AsBell`))) true))
  (set `self.SpawnerTimer` _returnvalue)
  (`self.SpawnMonster`))

(event `EndSpawning`
  ;[1 1 1] Stop spawning when shift ends
  (`KismetSystemLibrary.K2_ClearAndInvalidateTimerHandle` (`self.SpawnerTimer`)))

(event `SpawnMonster`
  (bind _totalmonsters (`self.TotalMonsters`))
  ;[1 1 1] Spawn monster
  (if (and (< _totalmonsters 5) (< _totalmonsters (`/Game/Blueprints/BP_ServiceBell.Level` (`self.AsBell`))))
    (bind _returnvalue (`|SpawnActorFromClass` "/Game/Blueprints/BP_Monster.BP_Monster_C" (`KismetMathLibrary.Conv_VectorToTransform` (`self.K2_GetActorLocation`)) "Undefined" "MultiplyWithRoot" null null))
    (set `self.AsMonster` _returnvalue)
    (set `self.TotalMonsters` (+ (`self.TotalMonsters`) 1))
    (set `/Game/Blueprints/BP_Monster.SpawnerPosition` (`self.K2_GetActorLocation`) (`self.AsMonster`))
    (add `/Game/Blueprints/BP_Monster.MonsterLeft` (`self.AsMonster`) (`|CreateDelegate` :!event `LowerTotalMonsters`))
    (bind (_valid _position) (`self.FindCounterPosition` :!label _label))
    (if _valid
      (set `/Game/Blueprints/BP_Monster.CounterPosition` _position (`self.AsMonster`))
      (`KismetArrayLibrary.Array_Set` (`self.CounterPositions`) _position true)
      (bind (_valid_2 _id) (`self.SelectMonsterId` :!label _label_2))
      (if _valid_2
        (`KismetArrayLibrary.Array_Add` (`self.MonsterIds`) _id)
        (set `/Game/Blueprints/BP_Monster.MonsterID` _id (`self.AsMonster`))
        (else
          (goto _label_2)))
      (else
        (goto _label)))))

(event `LowerTotalMonsters`
  (params (CounterPosition :type Integer) (ID :type Integer))
  ;[1 1 1] When monster leaves lower total monsters and remove array values
  (set `self.TotalMonsters` (- (`self.TotalMonsters`) 1))
  (`KismetArrayLibrary.Array_Set` (`self.CounterPositions`) CounterPosition)
  (`KismetArrayLibrary.Array_RemoveItem` (`self.MonsterIds`)))

(fn `FindCounterPosition`
  (returns (Valid :type Boolean) (Position :type Integer))
  (bind _returnvalue (`KismetMathLibrary.RandomIntegerInRange` 0 4))
  (return (not (`|GetArrayItem` (`self.CounterPositions`) _returnvalue)) _returnvalue))

(fn `SelectMonsterId`
  (returns (Valid :type Boolean) (ID :type Integer))
  (bind _returnvalue (`KismetMathLibrary.RandomIntegerInRange` 0 99))
  (for (_ _array_index) (`self.MonsterIds`)
    (if (== _array_index _returnvalue)
      (set `self.IdValid` false)
      (break)
      (else
        (set `self.IdValid` true))))
  (return (`self.IdValid`) _returnvalue))

(fn `UserConstructionScript`)