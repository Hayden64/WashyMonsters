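; Laundry customer monster that walks to its counter slot, gives the player dirty laundry, and awaits its return cleaned at a random temperature.
; Timers with progress-bar widgets track patience before handoff, then laundry time.
; A correct return pays money; a wrong one angers both this monster and the laundry's owner, damaging the player.
; Departing monsters show an emotion plane, walk to the spawner position, signal MonsterLeft and destroy themselves.
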(event `self.ReceiveBeginPlay`
  ;[1 1 1] Initialise
  (`KismetSystemLibrary.Delay` 0.1) ; Delay allows correct position to be set in Spawner
  (bind _asbp_player (cast `/Game/Blueprints/BP_Player` (`GameplayStatics.GetPlayerCharacter` 0)))
  (set `self.AsPlayer` _asbp_player)
  (`self.MoveToCounter`))

(event `MoveToCounter`
  ;[1 1 1] Move to counter
  (`|AIMoveTo` self (`KismetMathLibrary.MakeVector` -1200.0 (`KismetMathLibrary.Conv_IntToDouble` (* (+ (`self.CounterPosition`) 1) 275))) null
    (:`OnSuccess`
      (`self.WaitToBeServed`))))

(event `WaitToBeServed`
  (bind (_returnvalue_roll _returnvalue_pitch) (`KismetMathLibrary.BreakRotator` (`self.K2_GetActorRotation`)))
  ;[1 1 1] Wait to be served
  (bind _returnvalue (`KismetSystemLibrary.K2_SetTimerDelegate` (`|CreateDelegate` :!event `LeaveAngry`) (`self.PatienceTimerLength`))) ; Collect laundry before timer or monster leaves angry
  (set `self.PatienceTimer` _returnvalue)
  (bind _returnvalue_2 (`KismetSystemLibrary.K2_SetTimerDelegate` (`|CreateDelegate` :!event `UpdatePatienceTimerWidget`) 0.1 true))
  (set `self.UpdatePatienceWidgetTimer` _returnvalue_2)
  (bind _returnvalue_3 (`|GenericCreateObject` "/Game/Widgets/W_TimerBarRed.W_TimerBarRed_C"))
  (bind _output_get (set `self.AsPatienceTimerWidget` _returnvalue_3))
  (`WidgetComponent.SetWidget` (`self.PatienceTimerDisplay`) _output_get)
  (`SceneComponent.SetVisibility` (`self.PatienceTimerDisplay`) true false)
  (`self.K2_SetActorRotation` (`KismetMathLibrary.MakeRotator` _returnvalue_roll _returnvalue_pitch))
  (set `PrimitiveComponent.bGenerateOverlapEvents` true (`self.Box`)) ; Prevent interaction before monster is at desk
)

(event `/Game/Blueprints/I_Interact.Interact`
  (bind (_currentlaundry_owner _currentlaundry_laundrystate _currentlaundry_temperature) (break `/Game/Blueprints/S_Laundry` (`/Game/Blueprints/BP_Player.CurrentLaundry` (`self.AsPlayer`))))
  ;[1 1 1] Interact
  (switch `/Game/Blueprints/E_LaundryState` _currentlaundry_laundrystate
    (:`NewEnumerator0`
      (if (not (`self.HasGivenLaundry`))
        (set `/Game/Blueprints/BP_Player.CurrentLaundry` (make `/Game/Blueprints/S_Laundry` (`self.MonsterID`) "NewEnumerator1") (`self.AsPlayer`)) ; Give dirty laundry and owner
        (set `self.HasGivenLaundry` true)
        (`self.ChooseSpeech`)
        (`self.WaitForLaundry`)))
    (:`NewEnumerator3`
      (if (and (`|EnumEquality` (`self.DesiredTemperature`) _currentlaundry_temperature) (== _currentlaundry_owner (`self.MonsterID`)))
        (`self.LeaveHappy`)
        (else
          (`self.MakeOwnerLeaveAngry`)
          (`self.LeaveAngry`)))
      (set `/Game/Blueprints/BP_Player.CurrentLaundry` (make `/Game/Blueprints/S_Laundry` 0) (`self.AsPlayer`)) ; Remove laundry
    )))

(event `WaitForLaundry`
  (bind _tempdisplay (`self.TempDisplay`))
  ;[1 1 1] Show desired temp, set laundry timer
  (set `self.RandomForTemp` (`KismetMathLibrary.RandomIntegerInRange` 0 2))
  (`PrimitiveComponent.SetMaterial` _tempdisplay 0 (select `int` (`self.RandomForTemp`) :`0` "/Game/Materials/cold_Mat.cold_Mat" :`1` "/Game/Materials/medium_Mat.medium_Mat" :`2` "/Game/Materials/hot_Mat.hot_Mat" :!type "MaterialInterface Object Reference"))
  (set `self.DesiredTemperature` (select `int` (`self.RandomForTemp`) :`0` "NewEnumerator1" :`1` "NewEnumerator2" :`2` "NewEnumerator3" :!type "/Game/Blueprints/E_Temperature Enum"))
  (`SceneComponent.SetVisibility` _tempdisplay true false)
  (`KismetSystemLibrary.K2_ClearAndInvalidateTimerHandle` (`self.PatienceTimer`))
  (`KismetSystemLibrary.K2_ClearAndInvalidateTimerHandle` (`self.UpdatePatienceWidgetTimer`))
  (`SceneComponent.SetVisibility` (`self.PatienceTimerDisplay`) false false)
  (bind _returnvalue (`|GenericCreateObject` "/Game/Widgets/W_TimerBarBlue.W_TimerBarBlue_C"))
  (bind _output_get (set `self.AsLaundryTimerWidget` _returnvalue))
  (`WidgetComponent.SetWidget` (`self.LaundryTimerDisplay`) _output_get)
  (`SceneComponent.SetVisibility` (`self.LaundryTimerDisplay`) true false)
  (bind _returnvalue_2 (`KismetSystemLibrary.K2_SetTimerDelegate` (`|CreateDelegate` :!event `LeaveAngry`) (`self.LaundryTimerLength`))) ; Time to give correct laundry
  (set `self.LaundryTimer` _returnvalue_2)
  (bind _returnvalue_3 (`KismetSystemLibrary.K2_SetTimerDelegate` (`|CreateDelegate` :!event `UpdateLaundryTimerWidget`) 0.1 true))
  (set `self.UpdateLaundryWidgetTimer` _returnvalue_3))

(event `LeaveAngry`
  (bind (_returnvalue_x _returnvalue_y _returnvalue_z) (`KismetMathLibrary.BreakVector` (`self.K2_GetActorLocation`)))
  ;[1 1 1] Leave angrily
  (bind _returnvalue (`|SpawnActorFromClass` "/Game/Blueprints/BP_EmotionPlane.BP_EmotionPlane_C" (`KismetMathLibrary.MakeTransform` (`KismetMathLibrary.MakeVector` _returnvalue_x _returnvalue_y (+ _returnvalue_z 100.0)) (struct :`Yaw` 270.0 :`Roll` 90.0)) "Undefined" "MultiplyWithRoot" null null))
  (bind _output_get (set `self.AsEmotionPlane` _returnvalue))
  (`/Game/Blueprints/BP_EmotionPlane.DisplayEmoji` _output_get false)
  (`SceneComponent.SetVisibility` (`self.TempDisplay`) false false)
  (`GameplayStatics.ApplyDamage` (`self.AsPlayer`) 25.0)
  (`GameplayStatics.PlaySound2D` "/Game/Sounds/SFX/SFX_MonsterSad.SFX_MonsterSad" 1.0 1.0 0.0 null null)
  (`self.InvalidateAllTimers`)
  (`self.MoveToLeave`))

(event `LeaveHappy`
  (bind (_returnvalue_x _returnvalue_y _returnvalue_z) (`KismetMathLibrary.BreakVector` (`self.K2_GetActorLocation`)))
  (bind _asplayer (`self.AsPlayer`))
  ;[1 1 1] Leave happily
  (bind _returnvalue (`|SpawnActorFromClass` "/Game/Blueprints/BP_EmotionPlane.BP_EmotionPlane_C" (`KismetMathLibrary.MakeTransform` (`KismetMathLibrary.MakeVector` _returnvalue_x _returnvalue_y (+ _returnvalue_z 100.0)) (struct :`Yaw` 270.0 :`Roll` 90.0)) "Undefined" "MultiplyWithRoot" null null))
  (bind _output_get (set `self.AsEmotionPlane` _returnvalue))
  (`/Game/Blueprints/BP_EmotionPlane.DisplayEmoji` _output_get true)
  (`SceneComponent.SetVisibility` (`self.TempDisplay`) false false)
  (set `/Game/Blueprints/BP_Player.Money` (+ (`/Game/Blueprints/BP_Player.Money` _asplayer) 20.0) _asplayer)
  (`GameplayStatics.PlaySound2D` "/Game/Sounds/SFX/SFX_MonsterHappy.SFX_MonsterHappy" 1.0 1.0 0.0 null null)
  (`self.InvalidateAllTimers`)
  (`self.MoveToLeave`))

(event `MoveToLeave`
  ;[1 1 1] Leave when angry or happy
  (set `PrimitiveComponent.bGenerateOverlapEvents` false (`self.Box`)) ; Don't allow interaction when leaving
  (`|AIMoveTo` self (`self.SpawnerPosition`) null
    (:`OnSuccess`
      (`self.MonsterLeft` (`self.CounterPosition`) (`self.MonsterID`))
      (`KismetSystemLibrary.DelayUntilNextTick`)
      (`self.K2_DestroyActor`))))

(event `UpdatePatienceTimerWidget`
  ;[1 1 1] Update patience timer display
  (`ProgressBar.SetPercent` (`/Game/Widgets/W_TimerBarRed.ProgressBar` (`self.AsPatienceTimerWidget`)) (/ (`KismetSystemLibrary.K2_GetTimerRemainingTimeHandle` (`self.PatienceTimer`)) (`self.PatienceTimerLength`))))

(event `UpdateLaundryTimerWidget`
  ;[1 1 1] Update laundry timer display
  (`ProgressBar.SetPercent` (`/Game/Widgets/W_TimerBarBlue.ProgressBar` (`self.AsLaundryTimerWidget`)) (/ (`KismetSystemLibrary.K2_GetTimerRemainingTimeHandle` (`self.LaundryTimer`)) (`self.LaundryTimerLength`))))

(fn `ChooseSpeech`
  (`GameplayStatics.PlaySound2D` (select `int` (`KismetMathLibrary.RandomIntegerInRange` 0 5) :`0` "/Game/Sounds/SFX/SFX_MonsterTalk1.SFX_MonsterTalk1" :`1` "/Game/Sounds/SFX/SFX_MonsterTalk2.SFX_MonsterTalk2" :`2` "/Game/Sounds/SFX/SFX_MonsterTalk3.SFX_MonsterTalk3" :`3` "/Game/Sounds/SFX/SFX_MonsterTalk4.SFX_MonsterTalk4" :`4` "/Game/Sounds/SFX/SFX_MonsterTalk5.SFX_MonsterTalk5" :`5` "/Game/Sounds/SFX/SFX_MonsterTalk6.SFX_MonsterTalk6" :!type "SoundBase Object Reference") 1.0 (`KismetMathLibrary.RandomFloatInRange` 0.5 1.0) 0.0 null null))

(fn `InvalidateAllTimers`
  (`KismetSystemLibrary.K2_ClearAndInvalidateTimerHandle` (`self.PatienceTimer`))
  (`KismetSystemLibrary.K2_ClearAndInvalidateTimerHandle` (`self.UpdatePatienceWidgetTimer`))
  (`KismetSystemLibrary.K2_ClearAndInvalidateTimerHandle` (`self.LaundryTimer`))
  (`KismetSystemLibrary.K2_ClearAndInvalidateTimerHandle` (`self.UpdateLaundryWidgetTimer`)))

(fn `MakeOwnerLeaveAngry`
  (bind _currentlaundry_owner (break `/Game/Blueprints/S_Laundry` (`/Game/Blueprints/BP_Player.CurrentLaundry` (`self.AsPlayer`))))
  (bind _outactors (`GameplayStatics.GetAllActorsOfClass` "BP_Monster_C"))
  (for _array_element _outactors
    (if (== (`/Game/Blueprints/BP_Monster.MonsterID` _array_element) _currentlaundry_owner)
      (`self.LeaveAngry` _array_element)
      (break))))

(fn `UserConstructionScript`)