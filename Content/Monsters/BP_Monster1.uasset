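; BP_Monster1 is a laundry customer that hands over dirty washing and expects it back clean at a random temperature.
; It drives a blackboard MonsterState (Entering, Giving, Waiting, Leaving) and shows its demand or mood on a player-facing icon.
; Interact starts a widget-displayed timer, or matches a colon-delimited held-item string against LinePosition and Temperature to pay or damage the player.
; On destruction it may prompt the spawner to check customers.
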(event `self.ReceiveBeginPlay`
  (`KismetSystemLibrary.Delay` 0.5) ; Delay allows correct position to be set in Spawner
  (`BlackboardComponent.SetValueAsName` (`AIBlueprintHelperLibrary.GetBlackboard` null) "MonsterState" "Entering"))

(event `self.Box.OnComponentBeginOverlap`
  (params (OverlappedComponent :type "PrimitiveComponent Object Reference") (OtherActor :type "Actor Object Reference") (OtherComp :type "PrimitiveComponent Object Reference") (OtherBodyIndex :type Integer) (bFromSweep :type Boolean) (SweepResult :type "HitResult Structure (by ref)"))
  ;[1 0.4879 0.5277] Overlaps
)

(event `PresentWashing`
  (bind (_returnvalue_roll _returnvalue_pitch) (`KismetMathLibrary.BreakRotator` (`self.K2_GetActorRotation`)))
  (bind _emotion_temp (`self.Emotion/Temp`))
  ;[0.2701 1 0.1739] Waiting for player to take washing
  (switch `int` (`KismetMathLibrary.RandomIntegerInRange` 0 2)
    (:`0`
      (`PrimitiveComponent.SetMaterial` _emotion_temp 0 "/Game/Monsters/Assets/cold_Mat.cold_Mat")
      (set `self.Temperature` "Cold"))
    (:`1`
      (`PrimitiveComponent.SetMaterial` _emotion_temp 0 "/Game/Monsters/Assets/medium_Mat.medium_Mat")
      (set `self.Temperature` "Medium"))
    (:`2`
      (`PrimitiveComponent.SetMaterial` _emotion_temp 0 "/Game/Monsters/Assets/hot_Mat.hot_Mat")
      (set `self.Temperature` "Hot")))
  (`SceneComponent.SetVisibility` _emotion_temp true false)
  (`self.K2_SetActorRotation` (`KismetMathLibrary.MakeRotator` _returnvalue_roll _returnvalue_pitch))
  (set `PrimitiveComponent.bGenerateOverlapEvents` true (`self.Box`))
  (`BlackboardComponent.SetValueAsName` (`AIBlueprintHelperLibrary.GetBlackboard` null) "MonsterState" "Giving"))

(event `self.Box.OnComponentEndOverlap`
  (params (OverlappedComponent :type "PrimitiveComponent Object Reference") (OtherActor :type "Actor Object Reference") (OtherComp :type "PrimitiveComponent Object Reference") (OtherBodyIndex :type Integer))
  ;[1 0.4879 0.5277] Overlaps
)

(event `Leave angrily`
  (bind _emotion_temp (`self.Emotion/Temp`))
  ;[1 1 1] Leave angrily
  (bind _asbp_third_person_character (cast `/Game/ThirdPerson/Blueprints/BP_Player` (`GameplayStatics.GetPlayerCharacter` 0)))
  (`PrimitiveComponent.SetMaterial` _emotion_temp 0 "/Game/Monsters/Assets/Icon_Sad_Mat.Icon_Sad_Mat")
  (`SceneComponent.SetVisibility` _emotion_temp true false)
  (`GameplayStatics.ApplyDamage` _asbp_third_person_character 50.0)
  (`BlackboardComponent.SetValueAsName` (`AIBlueprintHelperLibrary.GetBlackboard` null) "MonsterState" "Leaving")
  (`GameplayStatics.PlaySound2D` "/Game/Felix/SFX_MonsterSad.SFX_MonsterSad" 1.0 1.0 0.0 null null))

(event `self.ReceiveTick`
  (params (DeltaSeconds :type "Float (single-precision)"))
  (bind _emotion_temp (`self.Emotion/Temp`))
  (bind _timer (`self.Timer`))
  ;[1 0.6408 0.8176] tick
  (if (not (not (`KismetSystemLibrary.K2_IsTimerActiveHandle` _timer)))
    (set `/Game/Monsters/WB_MonsterTimer.Timer Value` (/ (* (`KismetSystemLibrary.K2_GetTimerRemainingTimeHandle` _timer) 3.0) 100.0) (`self.TimerWidgetRef`)))
  (if (`SceneComponent.IsVisible` (`self.Emotion/Temp`))
    (bind _asbp_third_person_character (cast `/Game/ThirdPerson/Blueprints/BP_Player` (`GameplayStatics.GetPlayerCharacter` 0)))
    (bind (_returnvalue_roll _returnvalue_pitch _returnvalue_yaw) (`KismetMathLibrary.BreakRotator` (`KismetMathLibrary.FindLookAtRotation` (`SceneComponent.K2_GetComponentLocation` _emotion_temp) (`self.K2_GetActorLocation` _asbp_third_person_character))))
    (`SceneComponent.K2_SetWorldRotation` _emotion_temp (`KismetMathLibrary.MakeRotator` (+ _returnvalue_roll 90.0) 0.0 (- _returnvalue_yaw 90.0)) false false)))

(event `LeaveHappily`
  (bind _emotion_temp (`self.Emotion/Temp`))
  ;[1 1 1] Leave Happily
  (`KismetSystemLibrary.K2_PauseTimerHandle` (`self.Timer`))
  (bind _asbp_third_person_character (cast `/Game/ThirdPerson/Blueprints/BP_Player` (`GameplayStatics.GetPlayerCharacter` 0)))
  (`PrimitiveComponent.SetMaterial` _emotion_temp 0 "/Game/Monsters/Assets/Icon_Happy_Mat.Icon_Happy_Mat")
  (`SceneComponent.SetVisibility` _emotion_temp true false)
  (set `/Game/ThirdPerson/Blueprints/BP_Player.Money` (+ (`/Game/ThirdPerson/Blueprints/BP_Player.Money` _asbp_third_person_character) 20.0) _asbp_third_person_character)
  (`BlackboardComponent.SetValueAsName` (`AIBlueprintHelperLibrary.GetBlackboard` null) "MonsterState" "Leaving")
  (`GameplayStatics.PlaySound2D` "/Game/Felix/SFX_MonsterHappy.SFX_MonsterHappy" 1.0 1.0 0.0 null null))

(event `/Game/ThirdPerson/Blueprints/I_Interact.Interact`
  (bind _returnvalue (`KismetStringLibrary.Conv_IntToString` (`self.LinePosition`)))
  ;[1 1 1] Interact System, executed when called in the player class
  (bind _asbp_third_person_character (cast `/Game/ThirdPerson/Blueprints/BP_Player` (`GameplayStatics.GetPlayerCharacter` 0)))
  (bind _returnvalue_2 (`KismetStringLibrary.ParseIntoArray` (`/Game/ThirdPerson/Blueprints/BP_Player.Holding` _asbp_third_person_character) ":"))
  (if (== (`KismetArrayLibrary.Array_Length` _returnvalue_2) 3)
    (switch `string` (`|GetArrayItem` _returnvalue_2)
      (:`CleanLaundry`
        (if (and (`KismetStringLibrary.EqualEqual_StrStr` (`|GetArrayItem` _returnvalue_2 1) _returnvalue) (`KismetStringLibrary.EqualEqual_StrStr` (`|GetArrayItem` _returnvalue_2 2) (`self.Temperature`)))
          (`self.LeaveHappily`)
          (else
            (`self.Leave angrily`)))
        (set `/Game/ThirdPerson/Blueprints/BP_Player.Holding` "" _asbp_third_person_character)))
    (else
      (bind _output_get (set `/Game/ThirdPerson/Blueprints/BP_Player.Holding` (`KismetStringLibrary.Concat_StrStr` "DirtyLaundry:" _returnvalue) _asbp_third_person_character)) ; Hold item
      (`KismetSystemLibrary.PrintString` _output_get)
      (`BlackboardComponent.SetValueAsName` (`AIBlueprintHelperLibrary.GetBlackboard` null) "MonsterState" "Waiting")
      (bind _returnvalue_3 (`KismetSystemLibrary.K2_SetTimerDelegate` (`|CreateDelegate` :!event `Leave angrily`) 30.0))
      (set `self.Timer` _returnvalue_3)
      (bind _returnvalue_4 (`|GenericCreateObject` "/Game/Monsters/WB_MonsterTimer.WB_MonsterTimer_C"))
      (bind _output_get_2 (set `self.TimerWidgetRef` _returnvalue_4))
      (`WidgetComponent.SetWidget` (`self.TimerWidget`) _output_get_2))))

(event `self.ReceiveDestroyed`
  ;[1 1 1] Check on destroy if timer has expired
  (bind _returnvalue (`GameplayStatics.GetActorOfClass` "/Game/Monsters/A_MonsterSpawner.A_MonsterSpawner_C"))
  (if (not (`KismetSystemLibrary.K2_IsValidTimerHandle` (`/Game/Monsters/A_MonsterSpawner.SpawnerHandle` _returnvalue)))
    (`/Game/Monsters/A_MonsterSpawner.CheckCustomers` _returnvalue)))

(fn `UserConstructionScript`)