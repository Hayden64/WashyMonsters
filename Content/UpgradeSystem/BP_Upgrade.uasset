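; BP_Upgrade is an interactable machine-placement station where the player buys washing machines and dryers.
; Interact switches to a test camera, freezes player movement and opens W_PlaceMachine with mouse input; RemoveUI reverts this.
; Left click costs money and traces from the cursor, spawning the machine chosen by the Spawn flag at a Y-clamped, fixed-height point unless hitting another machine.
; The 180-degree flip logic is disconnected.
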(event `/Game/Blueprints/I_Interact.Interact`
  ;[0.6574 1 0.6224] Changes Camera (test whilst camera isnt fixed) - Hayden
  (bind _returnvalue (`GameplayStatics.GetActorOfClass` "/Game/UpgradeSystem/BP_CameraTest.BP_CameraTest_C"))
  (`PlayerController.SetViewTargetWithBlend` (`PlayerState.GetPlayerController` (`Pawn.PlayerState` (`GameplayStatics.GetPlayerCharacter` 0))) _returnvalue 0.0 "VTBlend_Linear" 0.0 false)
  (bind _returnvalue_2 (`GameplayStatics.GetActorOfClass` "/Game/Blueprints/BP_Player.BP_Player_C"))
  (set `/Game/Blueprints/BP_Player.CanMove` false _returnvalue_2)
  (bind _returnvalue_3 (`|CreateWidget` "/Game/UpgradeSystem/W_PlaceMachine.W_PlaceMachine_C" null self))
  (`UserWidget.AddToViewport` _returnvalue_3 0)
  (set `PlayerController.bShowMouseCursor` true (`GameplayStatics.GetPlayerController` 0))
  (`self.EnableInput` (`GameplayStatics.GetPlayerController` 0)))

(event `RemoveUI`
  ;[0.6574 1 0.6224] Reverts everything back to normal - Hayden
  (`Widget.RemoveFromParent` (stale `/Game/Blueprints/I_Interact.Interact` _returnvalue_3))
  (set `PlayerController.bShowMouseCursor` false (`GameplayStatics.GetPlayerController` 0))
  (bind _returnvalue (`GameplayStatics.GetActorOfClass` "/Game/Blueprints/BP_Player.BP_Player_C"))
  (set `/Game/Blueprints/BP_Player.CanMove` true _returnvalue)
  (bind _returnvalue_2 (`GameplayStatics.GetActorOfClass` "/Game/Blueprints/BP_Player.BP_Player_C"))
  (`PlayerController.SetViewTargetWithBlend` (`PlayerState.GetPlayerController` (`Pawn.PlayerState` (`GameplayStatics.GetPlayerCharacter` 0))) _returnvalue_2 0.0 "VTBlend_Linear" 0.0 false)
  (`self.DisableInput` (`GameplayStatics.GetPlayerController` 0)))

(event `Key|LeftMouseButton` :paused true
  (params (Key :type "Key Structure"))
  (bind _as_bp_third_person_character (`self.As BP Third Person Character`))
  (bind (_worldlocation _worlddirection) (`PlayerController.DeprojectMousePositionToWorld` (`GameplayStatics.GetPlayerController` 0)))
  (:`Pressed`
    ;[0.5891 1 0.5923] creates line trace from mouse location and places actor at the end of line trace - Hayden
    (bind _asbp_player (cast `/Game/Blueprints/BP_Player` (`GameplayStatics.GetPlayerCharacter` 0)))
    (bind _output_get (set `self.As BP Third Person Character` _asbp_player))
    ;;[0 0.003807 1] Can't place if money is less than 50
    (if (< (`/Game/Blueprints/BP_Player.Money` _output_get) 50.0)
      (`KismetSystemLibrary.PrintString` "Not enough money")
      (else
        (bind _outhit (`KismetSystemLibrary.LineTraceSingle` :`Start` _worldlocation :`End` (+ _worldlocation (* _worlddirection 5000000.0)) :`TraceChannel` "TraceTypeQuery1" :`DrawDebugType` "Persistent"))
        (cast `/Game/WashingMachineMinigame/BP_WashingMachine` (`.HitActor` (`GameplayStatics.BreakHitResult` _outhit))
          (:`CastFailed`
            (cast `/Game/DryerMinigame/BP_Dryer` (`.HitActor` (`GameplayStatics.BreakHitResult` _outhit))
              (:`CastFailed`
                (if (`self.Spawn`)
                  (bind _returnvalue (`KismetMathLibrary.FClamp` (.y (`.Location` (`GameplayStatics.BreakHitResult` _outhit))) -430.0 1270.0))
                  (`|SpawnActorFromClass` "/Game/WashingMachineMinigame/BP_WashingMachine.BP_WashingMachine_C" (`KismetMathLibrary.MakeTransform` (`KismetMathLibrary.MakeVector` (.x (`.Location` (`GameplayStatics.BreakHitResult` _outhit))) _returnvalue 70.0) (`KismetMathLibrary.MakeRotator` 0.0)) "Undefined" "MultiplyWithRoot" null null)
                  (else
                    (`|SpawnActorFromClass` "/Game/DryerMinigame/BP_Dryer.BP_Dryer_C" (`KismetMathLibrary.MakeTransform` (`KismetMathLibrary.MakeVector` (.x (`.Location` (`GameplayStatics.BreakHitResult` _outhit))) _returnvalue 70.0) (`KismetMathLibrary.MakeRotator` 0.0)) "Undefined" "MultiplyWithRoot" null null)))
                ;;[0 0.04334 1] Decreases money
                (set `/Game/Blueprints/BP_Player.Money` (- (`/Game/Blueprints/BP_Player.Money` _as_bp_third_person_character) 50.0) _as_bp_third_person_character)))))))))

(fn `UserConstructionScript`)