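; BP_ServiceBell is an interactable bell that starts a timed monster shift and advances the level when it ends.
; Interact lifts the bell out of the way, spawns a monster spawner and starts a one-minute timer shown on a level-timer widget.
; Timer expiry tells the spawner to stop spawning.
; Tick updates the countdown until the spawner becomes invalid, then increments the capped Level and lowers the bell back.
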(event `/Game/ThirdPerson/Blueprints/I_Interact.Interact`
  (bind (_returnvalue_x _returnvalue_y _returnvalue_z) (`KismetMathLibrary.BreakVector` (`self.K2_GetActorLocation`)))
  ;[1 1 1] Spawn monster spawner and start level timer
  (`self.K2_SetActorLocation` (`KismetMathLibrary.MakeVector` _returnvalue_x _returnvalue_y (+ _returnvalue_z 2000.0)))
  (bind _returnvalue (`|SpawnActorFromClass` "/Game/Monsters/A_MonsterSpawner.A_MonsterSpawner_C" (`KismetMathLibrary.MakeTransform` (-1600.0 240.0 0.0)) "Undefined" "MultiplyWithRoot" self null))
  (set `self.MonsterSpawnerRef` _returnvalue)
  (bind _returnvalue_2 (`KismetSystemLibrary.K2_SetTimerDelegate` (delegate `EndShift`) 60.0))
  (set `self.ShiftTimer` _returnvalue_2)
  (bind _returnvalue_3 (`|GenericCreateObject` "/Game/ServiceBell/WB_LevelTimer.WB_LevelTimer_C"))
  (bind _output_get (set `self.TimerWidgetRef` _returnvalue_3))
  (`WidgetComponent.SetWidget` (`self.TimerWidge`) _output_get)
  (set `self.ShiftStarted` true))

(event `EndShift`
  ;[1 1 1] Spawn monster spawner and start level timer
  (`/Game/Monsters/A_MonsterSpawner.EndSpawning` (`self.MonsterSpawnerRef`)))

(event `self.ReceiveTick`
  (params (DeltaSeconds :type "Float (single-precision)"))
  (bind (_returnvalue_x _returnvalue_y _returnvalue_z) (`KismetMathLibrary.BreakVector` (`self.K2_GetActorLocation`)))
  ;[1 1 1] Reset Level and increment
  (if (`self.ShiftStarted`)
    (if (`KismetSystemLibrary.IsValid` (`self.MonsterSpawnerRef`))
      (set `/Game/ServiceBell/WB_LevelTimer.TimerValue` (`KismetMathLibrary.FTrunc` (`KismetSystemLibrary.K2_GetTimerRemainingTimeHandle` (`self.ShiftTimer`))) (`self.TimerWidgetRef`))
      (else
        (set `self.ShiftStarted` false)
        (set `self.Level` (`KismetMathLibrary.FClamp` (+ (`self.Level`) 1.0) 1.0 3.0))
        (`self.K2_SetActorLocation` (`KismetMathLibrary.MakeVector` _returnvalue_x _returnvalue_y (- _returnvalue_z 2000.0)))))))

(fn `UserConstructionScript`)