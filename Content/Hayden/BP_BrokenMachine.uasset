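; BP_BrokenMachine is an interactable machine that opens the W_CleaningGame minigame widget.
; Interact creates the widget, shows the mouse cursor and blocks movement by clearing CanMove on BP_ThirdPersonCharacter.
; RemoveWidget reverses this by removing the widget, hiding the cursor and restoring movement; nothing in this Blueprint calls it.
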(event `/Game/ThirdPerson/Blueprints/I_Interact.Interact`
  ;[0.5819 1 0.5801] Adds widget to viewport and stops player from moving - Hayden
  (bind _returnvalue (`|CreateWidget` "/Game/Hayden/W_CleaningGame.W_CleaningGame_C"))
  (`UserWidget.AddToViewport` _returnvalue 0)
  (set `PlayerController.bShowMouseCursor` true (`GameplayStatics.GetPlayerController` 0))
  (bind _asbp_third_person_character (cast `/Game/ThirdPerson/Blueprints/BP_ThirdPersonCharacter` (`GameplayStatics.GetPlayerCharacter` 0)))
  (set `/Game/ThirdPerson/Blueprints/BP_ThirdPersonCharacter.CanMove` false _asbp_third_person_character))

(event `Remove Widget`
  ;[0.5318 1 0.5496] Removes the widget from the screen and allows the player to move - Hayden
  (`Widget.RemoveFromParent` (stale `/Game/ThirdPerson/Blueprints/I_Interact.Interact` _returnvalue))
  (set `PlayerController.bShowMouseCursor` false (`GameplayStatics.GetPlayerController` 0))
  (bind _asbp_third_person_character (cast `/Game/ThirdPerson/Blueprints/BP_ThirdPersonCharacter` (`GameplayStatics.GetPlayerCharacter` 0)))
  (set `/Game/ThirdPerson/Blueprints/BP_ThirdPersonCharacter.CanMove` true _asbp_third_person_character))

(fn `UserConstructionScript`)